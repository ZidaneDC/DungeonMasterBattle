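; Player controller that runs a prototype turn-based battle, spawning player and enemy units with random stats at spawn points and showing the battle HUD.
; Space in action select plays a round: living units attack random opponents in spawn order, as speed sorting is still a placeholder.
; Party KO checks trigger win or lose screens, and health variables mirror up to three units per side.
; Shift keys are debug kills for either team.
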(event Custom|SpawnAllies
  ;[1 1 1] Spawns player base class at all player spawn points, adds them to units and player units list. Assigns random stats to each
  (bind _outactors (Actor|GetAllActorsOfClass "/Game/BattleBP/Blueprints/Battle/PlayerSpawn.PlayerSpawn_C"))
  (for _array_element _outactors
    (bind _returnvalue (Game|SpawnActorfromClass "/Game/BattleBP/Blueprints/Battle/PlayerUnit.PlayerUnit_C" (Transformation|GetActorTransform _array_element) "Undefined" 0 0))
    (Development|PrintString "Allies Spawned!")
    (Utilities|Array|Add (Variables|Default|GetUnits) _returnvalue)
    (Utilities|Array|Add (Variables|Default|GetPlayerUnits) _returnvalue)
    (Default|SetStats _returnvalue)
    (Development|PrintString (Utilities|String|ToString(Integer) (Variables|/Game/BattleBP/Blueprints/Battle/BattleUnit_BaseClass.BattleUnit_BaseClass_C|GetSpeed _returnvalue)))))

(event Custom|SpawnEnemies
  ;[1 1 1] Spawns enemy base class at all enemy spawn points, adds them to units and enemy units list. Assigns random stats to each
  (bind _outactors (Actor|GetAllActorsOfClass "/Game/BattleBP/Blueprints/Battle/EnemySpawn.EnemySpawn_C"))
  (for _array_element _outactors
    (bind _returnvalue (Game|SpawnActorfromClass "/Game/BattleBP/Blueprints/Battle/EnemyUnit.EnemyUnit_C" (Transformation|GetActorTransform _array_element) "Undefined" 0 0))
    (Development|PrintString "Enemies Spawned!")
    (Utilities|Array|Add (Variables|Default|GetUnits) _returnvalue)
    (Utilities|Array|Add (Variables|Default|GetEnemyUnits) _returnvalue)
    (Default|SetStats _returnvalue)
    (Development|PrintString (Utilities|String|ToString(Integer) (Variables|/Game/BattleBP/Blueprints/Battle/BattleUnit_BaseClass.BattleUnit_BaseClass_C|GetSpeed _returnvalue)))))

(event Custom|BattleEnd
  ;[1 1 1] Check if the battle has ended and behaviour for if it has
  (bind (_isover _playerlost) (CallFunction|BattleEndCheck))
  (if _isover
    (if _playerlost
      (bind _returnvalue (UserInterface|CreateWidget "/Game/BattleBP/Blueprints/Battle/widgets/BattleLose.BattleLose_C"))
      (UserInterface|Viewport|AddtoViewport _returnvalue 0)
      (Variables|Default|Setstate "NewEnumerator4")
      (else
        (bind _returnvalue_2 (UserInterface|CreateWidget "/Game/BattleBP/Blueprints/Battle/widgets/BattleWin.BattleWin_C"))
        (UserInterface|Viewport|AddtoViewport _returnvalue_2 0)
        (Variables|Default|Setstate "NewEnumerator3")))
    (Development|PrintString "Battle has ended!")))

(event Custom|Enemy%20Health
  ;[1 0 0.032] Sets Health
  (for (_array_element _array_index) (Variables|Default|GetEnemyUnits)
    (if (== _array_index 0)
      (Variables|Default|SetenemyHeath1 (Math|Conversions|ToFloat(Integer) (Variables|/Game/BattleBP/Blueprints/Battle/BattleUnit_BaseClass.BattleUnit_BaseClass_C|GetCurrentHP _array_element)))
      (Utilities|FlowControl|DoOnce false
        (:Completed
          (Variables|Default|SetmaxEnemyHealth1 (Math|Conversions|ToFloat(Integer) (Variables|/Game/BattleBP/Blueprints/Battle/BattleUnit_BaseClass.BattleUnit_BaseClass_C|GetMaxHP _array_element)))))
      (elif (== _array_index 1)
        (Variables|Default|SetenemyHealth2 (Math|Conversions|ToFloat(Integer) (Variables|/Game/BattleBP/Blueprints/Battle/BattleUnit_BaseClass.BattleUnit_BaseClass_C|GetCurrentHP _array_element)))
        (Utilities|FlowControl|DoOnce false
          (:Completed
            (Variables|Default|SetmaxEnemyHealth2 (Math|Conversions|ToFloat(Integer) (Variables|/Game/BattleBP/Blueprints/Battle/BattleUnit_BaseClass.BattleUnit_BaseClass_C|GetMaxHP _array_element)))))
        (elif (== _array_index 2)
          (Variables|Default|SetenemyHealth3 (Math|Conversions|ToFloat(Integer) (Variables|/Game/BattleBP/Blueprints/Battle/BattleUnit_BaseClass.BattleUnit_BaseClass_C|GetCurrentHP _array_element)))
          (Utilities|FlowControl|DoOnce false
            (:Completed
              (Variables|Default|SetmaxEnemyHealth3 (Math|Conversions|ToFloat(Integer) (Variables|/Game/BattleBP/Blueprints/Battle/BattleUnit_BaseClass.BattleUnit_BaseClass_C|GetMaxHP _array_element))))))))))

(event Custom|Player%20Health
  ;[1 0 0.032] Sets Health
  (for (_array_element _array_index) (Variables|Default|GetPlayerUnits)
    (if (== _array_index 0)
      (Variables|Default|SetplayerHealth1 (Math|Conversions|ToFloat(Integer) (Variables|/Game/BattleBP/Blueprints/Battle/BattleUnit_BaseClass.BattleUnit_BaseClass_C|GetCurrentHP _array_element)))
      (Utilities|FlowControl|DoOnce false
        (:Completed
          (Variables|Default|SetmaxPlayerHealth1 (Math|Conversions|ToFloat(Integer) (Variables|/Game/BattleBP/Blueprints/Battle/BattleUnit_BaseClass.BattleUnit_BaseClass_C|GetMaxHP _array_element)))))
      (elif (== _array_index 1)
        (Variables|Default|SetplayerHealth2 (Math|Conversions|ToFloat(Integer) (Variables|/Game/BattleBP/Blueprints/Battle/BattleUnit_BaseClass.BattleUnit_BaseClass_C|GetCurrentHP _array_element)))
        (Utilities|FlowControl|DoOnce false
          (:Completed
            (Variables|Default|SetmaxPlayerHealth2 (Math|Conversions|ToFloat(Integer) (Variables|/Game/BattleBP/Blueprints/Battle/BattleUnit_BaseClass.BattleUnit_BaseClass_C|GetMaxHP _array_element)))))
        (elif (== _array_index 2)
          (Variables|Default|SetplayerHealth3 (Math|Conversions|ToFloat(Integer) (Variables|/Game/BattleBP/Blueprints/Battle/BattleUnit_BaseClass.BattleUnit_BaseClass_C|GetCurrentHP _array_element)))
          (Utilities|FlowControl|DoOnce false
            (:Completed
              (Variables|Default|SetmaxPlayerHealth3 (Math|Conversions|ToFloat(Integer) (Variables|/Game/BattleBP/Blueprints/Battle/BattleUnit_BaseClass.BattleUnit_BaseClass_C|GetMaxHP _array_element))))))))))

(event EventBeginPlay
  (bind _returnvalue (UserInterface|CreateWidget "/Game/BattleBP/Blueprints/UI/BattleHud.BattleHud_C"))
  (UserInterface|Viewport|AddtoViewport _returnvalue 0)
  (CallFunction|SpawnAllies)
  (CallFunction|SpawnEnemies)
  (CallFunction|EnemyHealth)
  (CallFunction|PlayerHealth)
  (Utilities|FlowControl|Delay 2.0))

(event Input|KeyboardEvents|LeftShift
  (params (Key :type Key%20Structure :default "None"))
  ;[1 1 1] DEBUG ONLY kill all commands to end a battle
  (:Pressed
    (CallFunction|KillAllPlayer)
    (CallFunction|BattleEnd)))

(event Input|KeyboardEvents|RightShift
  (params (Key :type Key%20Structure :default "None"))
  ;[1 1 1] DEBUG ONLY kill all commands to end a battle
  (:Pressed
    (CallFunction|KillAllEnemy)
    (CallFunction|BattleEnd)))

(event Input|KeyboardEvents|Enter
  (params (Key :type Key%20Structure :default "None"))
  ;[1 1 1] Behaviour when spacebar/enter is pressed depending on player state
)

(event Input|KeyboardEvents|SpaceBar
  (params (Key :type Key%20Structure :default "None"))
  ;[1 1 1] Behaviour when spacebar/enter is pressed depending on player state
  (:Pressed
    (switch Utilities|FlowControl|Switch|SwitchonPlayerState_Battle (Variables|Default|Getstate)
      (:NewEnumerator5
        (bind _turnorder (CallFunction|DetermineTurnOrder))
        (bind _isbattleover (CallFunction|BeginTurns _turnorder))
        (CallFunction|EnemyHealth)
        (CallFunction|PlayerHealth)
        (if _isbattleover
          (CallFunction|BattleEnd)
          (else
            (Variables|Default|Setstate "NewEnumerator5")))))))

(fn ConstructionScript)

(fn BeginTurns
  (params (TurnOrder :type Array%20of%20Battle%20Unit%20Base%20Class%20Object%20References))
  (Development|PrintString "Turn Initiated!")
  (bind _array_element (Utilities|Array|ForEachLoopwithBreak TurnOrder)
    (:LoopBody
      (bind _isplayerturn (CallFunction|CheckifPlayerTurn _array_element))
      (if _isplayerturn
        (CallFunction|PlayerTurn _array_element)
        (else
          (CallFunction|EnemyTurn _array_element)))
      (bind _isover (CallFunction|BattleEndCheck))
      (if _isover
        (return _isover)))
    (:Completed
      (return _isover))))

(fn DetermineTurnOrder
  ;[1 1 1] determines what order units go in, Currently placeholder, does not sort by speed and simply copies units array instead
  (Utilities|Array|Clear (Variables|Default|GetTurnOrder)) ; Clear the array from last turn
  (Development|PrintString "Turn Order:")
  (for _array_element (Variables|Default|GetUnits)
    (if (not (Variables|/Game/BattleBP/Blueprints/Battle/BattleUnit_BaseClass.BattleUnit_BaseClass_C|GetisDead _array_element))
      (Development|PrintString (Utilities|GetDisplayName _array_element))
      (Utilities|Array|Add (Variables|Default|GetTurnOrder) _array_element)))
  (return (Variables|Default|GetTurnOrder)))

(fn PlayerTurn
  (params (Attacker :type Battle%20Unit%20Base%20Class%20Object%20Reference))
  (Variables|Default|Setstate "NewEnumerator1")
  (if (not (Variables|/Game/BattleBP/Blueprints/Battle/BattleUnit_BaseClass.BattleUnit_BaseClass_C|GetisDead Attacker))
    (Development|PrintString "Players turn!")
    ;[1 1 1] placeholder section, this should access an array of that character's actions for that turn and execute each
    (bind _selectedtarget (CallFunction|RandomSelect false))
    (CallFunction|ExecuteAttack Attacker _selectedtarget)))

(fn EnemyTurn
  (params (Attacker :type Battle%20Unit%20Base%20Class%20Object%20Reference))
  (Variables|Default|Setstate "NewEnumerator0")
  (if (not (Variables|/Game/BattleBP/Blueprints/Battle/BattleUnit_BaseClass.BattleUnit_BaseClass_C|GetisDead Attacker))
    (Development|PrintString "Enemy turn!")
    (bind _selectedtarget (CallFunction|RandomSelect true))
    (CallFunction|ExecuteAttack Attacker _selectedtarget)))

(fn BattleEndCheck
  (bind _ispartyko_d (CallFunction|PartyKOCheck (Variables|Default|GetPlayerUnits)))
  (if _ispartyko_d
    (return true true)
    (else
      (bind _ispartyko_d_2 (CallFunction|PartyKOCheck (Variables|Default|GetEnemyUnits)))
      (if _ispartyko_d_2
        (Development|PrintString "battle is over!")
        (return true false)
        (else
          (Development|PrintString "battle is not over")
          (return false false))))))

(fn PartyKOCheck
  (params (Party :type Array%20of%20Battle%20Unit%20Base%20Class%20Object%20References))
  (bind _array_element (Utilities|Array|ForEachLoopwithBreak Party)
    (:LoopBody
      (if (not (<= (Variables|/Game/BattleBP/Blueprints/Battle/BattleUnit_BaseClass.BattleUnit_BaseClass_C|GetCurrentHP _array_element) 0))
        (bind _output_get (LocalVariables|SetIsPartyDead false))
        (return _output_get) ; if any party member is alive, return immediately as false
      ))
    (:Completed
      (Development|PrintString "Party is KO'd!")
      (bind _output_get_2 (LocalVariables|SetIsPartyDead true))
      (return _output_get_2))))

(fn CheckifPlayerTurn
  (params (Unit :type Battle%20Unit%20Base%20Class%20Object%20Reference))
  (if (Variables|/Game/BattleBP/Blueprints/Battle/BattleUnit_BaseClass.BattleUnit_BaseClass_C|GetisPlayer Unit)
    (return true)
    (else
      (return false))))

(fn ExecuteAttack
  (params (Attacker :type Battle%20Unit%20Base%20Class%20Object%20Reference) (Defender :type Battle%20Unit%20Base%20Class%20Object%20Reference))
  (bind _damagedealt (Default|TakeDamage Defender Attacker))
  (Development|PrintString (Utilities|GetDisplayName Attacker))
  (Development|PrintString "does")
  (Development|PrintString (Utilities|String|ToString(Integer) _damagedealt))
  (Development|PrintString "damage to")
  (Development|PrintString (Utilities|GetDisplayName Defender))
  (Default|DeathCheck Defender) ; check if the target is dead
)

(fn RandomSelect
  (params (IsAttackingPlayer :type Boolean))
  (bind _selectableunits (LocalVariables|GetSelectableUnits))
  (if IsAttackingPlayer
    ;[1 1 1] choose from player character units
    (for _array_element (Variables|Default|GetPlayerUnits)
      (if (not (Variables|/Game/BattleBP/Blueprints/Battle/BattleUnit_BaseClass.BattleUnit_BaseClass_C|GetisDead _array_element))
        (Utilities|Array|Add (LocalVariables|GetSelectableUnits) _array_element)))
    (else
      ;[1 1 1] choose from enemy units
      (for _array_element_2 (Variables|Default|GetEnemyUnits)
        (if (not (Variables|/Game/BattleBP/Blueprints/Battle/BattleUnit_BaseClass.BattleUnit_BaseClass_C|GetisDead _array_element_2))
          (Utilities|Array|Add (LocalVariables|GetSelectableUnits) _array_element_2)))))
  (bind _output_get (LocalVariables|SetSelectedUnit (Utilities|Array|Get(acopy) _selectableunits (Math|Random|RandomInteger (Utilities|Array|Length _selectableunits)))))
  (return _output_get))

(fn KillAllPlayer
  ;[1 1 1] DEBUG ONLY
  (for _array_element (Variables|Default|GetPlayerUnits)
    (Variables|/Game/BattleBP/Blueprints/Battle/BattleUnit_BaseClass.BattleUnit_BaseClass_C|SetCurrentHP _array_element 0)
    (Default|DeathCheck _array_element)))

(fn KillAllEnemy
  ;[1 1 1] DEBUG ONLY
  (for _array_element (Variables|Default|GetEnemyUnits)
    (Variables|/Game/BattleBP/Blueprints/Battle/BattleUnit_BaseClass.BattleUnit_BaseClass_C|SetCurrentHP _array_element 0)
    (Default|DeathCheck _array_element)))
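; CardDamageCalc is a battle Blueprint that scores player and enemy card hands as damage and decides who gets hurt.
; CheckSameColor adds a bonus for two or three cards of the majority color.
; CompareDmg stores the difference between both totals and flags whether the player takes it, and ResetCardsDmg clears hands and values.
; CalcDmg, sorting, summing, straight, three-of-a-kind and pair functions are empty stubs.
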(event EventBeginPlay)

(event EventTick
  (params (DeltaSeconds :type Float%20%28single-precision%29)))

(fn CalcDmg)

(fn SortCards
  (params (Cards :type Array%20of%20Action%20Data%20Asset%20Object%20References)))

(fn AddCardsUp
  (params (Cards :type Array%20of%20Action%20Data%20Asset%20Object%20References) (DmgValue :type Integer)))

(fn CheckforStraight
  (params (Cards :type Array%20of%20Action%20Data%20Asset%20Object%20References)))

(fn Checkif3OfAKind
  (params (Cards :type Array%20of%20Action%20Data%20Asset%20Object%20References)))

(fn CheckifPair
  (params (Cards :type Array%20of%20Action%20Data%20Asset%20Object%20References) (DmgValue :type Integer)))

(fn CheckSameColor
  (params (Cards :type Array%20of%20Action%20Data%20Asset%20Object%20References) (DmgValue :type Integer))
  (LocalVariables|SetDmgValueCalculated DmgValue)
  (for _array_element Cards
    (switch string (Variables|/Game/BattleBP/Blueprints/Actions/ActionDataAsset.ActionDataAsset_C|GetColor _array_element)
      (:Red
        (Math|Integer|IncrementInt (LocalVariables|GetNumRed)))
      (:Black
        (Math|Integer|IncrementInt (LocalVariables|GetNumBlack)))))
  (if (> (LocalVariables|GetNumRed) (LocalVariables|GetNumBlack))
    (switch int (LocalVariables|GetNumRed)
      (:Default
        _)
      (:2
        (bind _output_get (LocalVariables|SetDmgValueCalculated (+ (LocalVariables|GetDmgValueCalculated) 3)))
        (return _output_get))
      (:3
        (bind _output_get_2 (LocalVariables|SetDmgValueCalculated (+ (LocalVariables|GetDmgValueCalculated) 5)))
        (return _output_get_2)))
    (else
      (switch int (LocalVariables|GetNumBlack)
        (:Default
          _)
        (:2
          (bind _output_get_3 (LocalVariables|SetDmgValueCalculated (+ (LocalVariables|GetDmgValueCalculated) 3)))
          (return _output_get_3))
        (:3
          (bind _output_get_4 (LocalVariables|SetDmgValueCalculated (+ (LocalVariables|GetDmgValueCalculated) 5)))
          (return _output_get_4)))))
  (return (LocalVariables|GetDmgValueCalculated)))

(fn CompareDmg
  (if (> (Variables|Default|GetPlayerDmg) (Variables|Default|GetEnemyDmg))
    (Variables|Default|SetDmgDealt (- (Variables|Default|GetPlayerDmg) (Variables|Default|GetEnemyDmg)))
    (Variables|Default|SetIsPlayerTakingDmg false)
    (elif (< (Variables|Default|GetPlayerDmg) (Variables|Default|GetEnemyDmg))
      (Variables|Default|SetDmgDealt (- (Variables|Default|GetEnemyDmg) (Variables|Default|GetPlayerDmg)))
      (Variables|Default|SetIsPlayerTakingDmg true)
      (elif (== (Variables|Default|GetEnemyDmg) (Variables|Default|GetPlayerDmg))
        (Variables|Default|SetDmgDealt 0)))))

(fn ResetCards&Dmg
  (Utilities|Array|Clear (Variables|Default|GetPlayersCards))
  (Utilities|Array|Clear (Variables|Default|GetEnemyCards))
  (Variables|Default|SetPlayerDmg 0)
  (Variables|Default|SetEnemyDmg 0)
  (Variables|Default|SetDmgDealt 0))
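; Base battle unit for a turn-based battle system, holding Speed, Attack, Defense and HP with placeholder logic.
; SetStats randomizes the stats and fills current HP to max.
; TakeDamage subtracts attacker Attack minus own Defense from HP without clamping, and a separate DeathCheck hides the actor and prints a KO message at zero or below.
; ShowIndicator, despite its name, hides the Indicator component.
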(event Custom|SetStats
  (CallFunction|AssignRandomStats))

(fn ConstructionScript)

(fn DeathCheck
  (if (<= (Variables|Stats|GetCurrentHP) 0)
    (Variables|Default|SetisDead true)
    (Rendering|SetActorHiddenInGame true)
    (Development|PrintString (Utilities|GetDisplayName self))
    (Development|PrintString " is KO'd!")
    (else
      (Variables|Default|SetisDead false))))

(fn AssignRandomStats
  (bind _returnvalue (Math|Random|RandomIntegerinRange 10 20))
  (bind _returnvalue_2 (Math|Random|RandomIntegerinRange 1 20))
  (Variables|Stats|SetSpeed _returnvalue)
  (Variables|Stats|SetAttack _returnvalue)
  (Variables|Stats|SetDefense _returnvalue_2)
  (bind _output_get (Variables|Stats|SetMaxHP _returnvalue_2))
  (Variables|Stats|SetCurrentHP _output_get))

(fn TakeDamage
  (params (Attacker :type Battle%20Unit%20Base%20Class%20Object%20Reference))
  ;[1 1 1] placeholder damage calculation
  (bind _output_get (Variables|Stats|SetCurrentHP (- (Variables|Stats|GetCurrentHP) (- (Variables|BattleUnit_BaseClass_C|GetAttack Attacker) (Variables|Stats|GetDefense)))))
  (return _output_get))

(fn ShowIndicator
  (Rendering|SetVisibility (Variables|Default|GetIndicator) false false))
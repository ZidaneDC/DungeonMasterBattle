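; Turn-based battle manager that spawns player and enemy units at spawn points and runs their attacks.
; Turn order is rebuilt from living units in spawn order, a placeholder for speed sorting.
; BeginTurns loops a whole round with win/loss checks, while NextTurn steps through units by index.
; Both sides attack random targets as a targeting placeholder; SelectableUnits is never cleared here between picks.
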(event Custom|SpawnAllies_Event
  ;[1 1 1] Spawns player base class at all player spawn points, adds them to units and player units list. Assigns random stats to each
  (bind _outactors (Actor|GetAllActorsOfClass "/Game/BattleBP/Blueprints/Battle/PlayerSpawn.PlayerSpawn_C"))
  (for _array_element _outactors
    (bind _returnvalue (Game|SpawnActorfromClass "/Game/BattleBP/Blueprints/Battle/PlayerUnit.PlayerUnit_C" (Transformation|GetActorTransform _array_element) "Undefined" 0 0))
    (Development|PrintString "Allies Spawned!")
    (Utilities|Array|Add (Variables|Default|GetUnits) _returnvalue)
    (Utilities|Array|Add (Variables|Default|GetPlayerUnits) _returnvalue)
    (Default|SetStats _returnvalue)
    (Development|PrintString (Utilities|String|ToString(Integer) (Variables|/Game/BattleBP/Blueprints/Battle/BattleUnit_BaseClass.BattleUnit_BaseClass_C|GetSpeed _returnvalue)))))

(event Custom|SpawnEnemies_Event
  ;[1 1 1] Spawns enemy base class at all enemy spawn points, adds them to units and enemy units list. Assigns random stats to each
  (bind _outactors (Actor|GetAllActorsOfClass "/Game/BattleBP/Blueprints/Battle/EnemySpawn.EnemySpawn_C"))
  (for _array_element _outactors
    (bind _returnvalue (Game|SpawnActorfromClass "/Game/BattleBP/Blueprints/Battle/EnemyUnit.EnemyUnit_C" (Transformation|GetActorTransform _array_element) "Undefined" 0 0))
    (Development|PrintString "Enemies Spawned!")
    (Utilities|Array|Add (Variables|Default|GetUnits) _returnvalue)
    (Utilities|Array|Add (Variables|Default|GetEnemyUnits) _returnvalue)
    (Default|SetStats _returnvalue)
    (Development|PrintString (Utilities|String|ToString(Integer) (Variables|/Game/BattleBP/Blueprints/Battle/BattleUnit_BaseClass.BattleUnit_BaseClass_C|GetSpeed _returnvalue)))))

(event EventBeginPlay
  (bind _asbattle_player_controller (Utilities|Casting|CastToBattlePlayerController (Game|Player|GetPlayerPawn 0)))
  (Variables|Default|SetPlayer _asbattle_player_controller))

(fn DetermineTurnOrder
  ;[1 1 1] determines what order units go in, Currently placeholder, does not sort by speed and simply copies units array instead
  (Utilities|Array|Clear (Variables|Default|GetTurnOrder)) ; Clear the array from last turn
  (Variables|Default|SetCurrCharacterIndex 0)
  (Development|PrintString "Turn Order:")
  (for _array_element (Variables|Default|GetUnits)
    (if (not (Variables|/Game/BattleBP/Blueprints/Battle/BattleUnit_BaseClass.BattleUnit_BaseClass_C|GetisDead _array_element))
      (Development|PrintString (Utilities|GetDisplayName _array_element))
      (Utilities|Array|Add (Variables|Default|GetTurnOrder) _array_element)))
  (return (Variables|Default|GetTurnOrder)))

(fn BattleEndCheck
  (bind _ispartyko_d (CallFunction|PartyKOCheck (Variables|Default|GetPlayerUnits)))
  (if _ispartyko_d
    (return true true)
    (else
      (bind _ispartyko_d_2 (CallFunction|PartyKOCheck (Variables|Default|GetEnemyUnits)))
      (if _ispartyko_d_2
        (Development|PrintString "battle is over!")
        (return true false)
        (else
          (Development|PrintString "battle is not over")
          (return false false))))))

(fn PartyKOCheck
  (params (Party :type Array%20of%20Battle%20Unit%20Base%20Class%20Object%20References))
  (bind _array_element (Utilities|Array|ForEachLoopwithBreak Party)
    (:LoopBody
      (if (not (<= (Variables|/Game/BattleBP/Blueprints/Battle/BattleUnit_BaseClass.BattleUnit_BaseClass_C|GetCurrentHP _array_element) 0))
        (bind _output_get (LocalVariables|SetisPartyDead false))
        (return _output_get) ; if any party member is alive, return immediately as false
      ))
    (:Completed
      (Development|PrintString "Party is KO'd!")
      (bind _output_get_2 (LocalVariables|SetisPartyDead true))
      (return _output_get_2))))

(fn CheckifPlayerTurn
  (params (Unit :type Battle%20Unit%20Base%20Class%20Object%20Reference))
  (if (Variables|/Game/BattleBP/Blueprints/Battle/BattleUnit_BaseClass.BattleUnit_BaseClass_C|GetisPlayer Unit)
    (return true)
    (else
      (return false))))

(fn ExecuteAttack
  (params (Attacker :type Battle%20Unit%20Base%20Class%20Object%20Reference) (Defender :type Battle%20Unit%20Base%20Class%20Object%20Reference))
  (bind _damagedealt (Default|TakeDamage Defender Attacker))
  (Development|PrintString (Utilities|GetDisplayName Attacker))
  (Development|PrintString "does")
  (Development|PrintString (Utilities|String|ToString(Integer) _damagedealt))
  (Development|PrintString "damage to")
  (Development|PrintString (Utilities|GetDisplayName Defender))
  (Default|DeathCheck Defender) ; check if the target is dead
)

(fn RandomSelect
  (params (isAttackingPlayer :type Boolean))
  (bind _selectableunits (LocalVariables|GetSelectableUnits))
  (if isAttackingPlayer
    ;[1 1 1] choose from player character units
    (for _array_element (Variables|Default|GetPlayerUnits)
      (if (not (Variables|/Game/BattleBP/Blueprints/Battle/BattleUnit_BaseClass.BattleUnit_BaseClass_C|GetisDead _array_element))
        (Utilities|Array|Add (LocalVariables|GetSelectableUnits) _array_element)))
    (else
      ;[1 1 1] choose from enemy units
      (for _array_element_2 (Variables|Default|GetEnemyUnits)
        (if (not (Variables|/Game/BattleBP/Blueprints/Battle/BattleUnit_BaseClass.BattleUnit_BaseClass_C|GetisDead _array_element_2))
          (Utilities|Array|Add (LocalVariables|GetSelectableUnits) _array_element_2)))))
  (bind _output_get (LocalVariables|SetSelectedUnit (Utilities|Array|Get(acopy) _selectableunits (Math|Random|RandomInteger (Utilities|Array|Length _selectableunits)))))
  (return _output_get))

(fn PlayerTurn
  (params (Attacker :type Battle%20Unit%20Base%20Class%20Object%20Reference))
  (Variables|/Game/BattleBP/Blueprints/BattlePlayerController.BattlePlayerController_C|Setstate (Variables|Default|GetPlayer) "NewEnumerator1")
  (if (Variables|/Game/BattleBP/Blueprints/Battle/BattleUnit_BaseClass.BattleUnit_BaseClass_C|GetisDead Attacker)
    (bind _result (Math|Integer|IncrementInt (Variables|Default|GetCurrCharacterIndex))
      (:%20%20
        (Variables|Default|SetCurrCharacterIndex _result)
        (CallFunction|NextTurn)))
    (else
      (Development|PrintString "Players turn!")
      ;[1 1 1] placeholder section, this should show menu UI and allow the player to choose an action
      (bind _selectedtarget (CallFunction|RandomSelect false))
      (CallFunction|ExecuteAttack Attacker _selectedtarget)
      (bind _result_2 (Math|Integer|IncrementInt (Variables|Default|GetCurrCharacterIndex))
        (:%20%20
          (Variables|Default|SetCurrCharacterIndex _result_2))))))

(fn EnemyTurn
  (params (Attacker :type Battle%20Unit%20Base%20Class%20Object%20Reference))
  (Variables|/Game/BattleBP/Blueprints/BattlePlayerController.BattlePlayerController_C|Setstate (Variables|Default|GetPlayer) "NewEnumerator0")
  (if (Variables|/Game/BattleBP/Blueprints/Battle/BattleUnit_BaseClass.BattleUnit_BaseClass_C|GetisDead Attacker)
    (bind _result (Math|Integer|IncrementInt (Variables|Default|GetCurrCharacterIndex))
      (:%20%20
        (Variables|Default|SetCurrCharacterIndex _result)
        (CallFunction|NextTurn)))
    (else
      (Development|PrintString "Enemy turn!")
      (bind _selectedtarget (CallFunction|RandomSelect true))
      (CallFunction|ExecuteAttack Attacker _selectedtarget)
      (bind _result_2 (Math|Integer|IncrementInt (Variables|Default|GetCurrCharacterIndex))
        (:%20%20
          (Variables|Default|SetCurrCharacterIndex _result_2))))))

(fn BeginTurns
  (params (TurnOrder :type Array%20of%20Battle%20Unit%20Base%20Class%20Object%20References))
  (Development|PrintString "Turn Initiated")
  (bind _array_element (Utilities|Array|ForEachLoopwithBreak TurnOrder)
    (:LoopBody
      (bind _isplayerturn (CallFunction|CheckifPlayerTurn _array_element))
      (if _isplayerturn
        (CallFunction|PlayerTurn _array_element)
        (else
          (CallFunction|EnemyTurn _array_element)))
      (bind _isover (CallFunction|BattleEndCheck))
      (if _isover
        (return _isover)))
    (:Completed
      (return _isover))))

(fn KillAllPlayer
  (for _array_element (Variables|Default|GetPlayerUnits)
    (Variables|/Game/BattleBP/Blueprints/Battle/BattleUnit_BaseClass.BattleUnit_BaseClass_C|SetCurrentHP _array_element 0)
    (Default|DeathCheck _array_element)))

(fn KillAllEnemy
  (for _array_element (Variables|Default|GetEnemyUnits)
    (Variables|/Game/BattleBP/Blueprints/Battle/BattleUnit_BaseClass.BattleUnit_BaseClass_C|SetCurrentHP _array_element 0)
    (Default|DeathCheck _array_element)))

(fn NextTurn
  (bind _turnorder (Variables|Default|GetTurnOrder))
  (bind _currcharacterindex (Variables|Default|GetCurrCharacterIndex))
  (bind _output (Utilities|Array|Get(acopy) _turnorder _currcharacterindex))
  (if (< (Utilities|Array|LastIndex (Variables|Default|GetTurnOrder)) (Variables|Default|GetCurrCharacterIndex))
    (CallFunction|DetermineTurnOrder))
  (bind _isplayerturn (CallFunction|CheckifPlayerTurn _output))
  (if _isplayerturn
    (CallFunction|PlayerTurn _output)
    (else
      (CallFunction|EnemyTurn _output))))
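; Turn-based battle game mode that alternates turns between two player controller indices.
; The match starts when player count reaches one on PostLogin, calling StartTurn on the current PlayerController_Battle.
; CycleTurn ends that controller's turn, flips the index between 0 and 1, then starts the other's.
; ChoosePlayerStart lazily maps TurnBasedPlayerStart actors by player index and picks the one keyed by current player count.
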(event Custom|StartMatch
  (Default|StartTurn (Utilities|PlayerTurn)))

(event Custom|CycleTurn
  (Default|EndTurn (Utilities|PlayerTurn))
  (Variables|Default|SetcurrPlayerTurn (select (== (Variables|Default|GetcurrPlayerTurn) 0) 1 0))
  (Default|StartTurn (Utilities|PlayerTurn)))

(event EventPostLogin
  (params (NewPlayer :type Player%20Controller%20Object%20Reference))
  (bind _returnvalue (Class|GameModeBase|GetNumPlayers))
  (if (== _returnvalue 1)
    (CallFunction|StartMatch)))

(fn ConstructionScript)

(fn ChoosePlayerStart
  (params (Player :type Controller%20Object%20Reference))
  (CallFunction|InitializeSpawn)
  (bind _returnvalue (Class|GameModeBase|GetNumPlayers))
  (return (.Value (Utilities|Map|Find (Variables|Default|GetSpawnPoints) _returnvalue))))

(fn InitializeSpawn
  (if (== (Utilities|Map|Length (Variables|Default|GetSpawnPoints)) 0)
    (bind _outactors (Actor|GetAllActorsOfClass "/Game/BattleBP/Blueprints/Battle/TurnBasedPlayerStart.TurnBasedPlayerStart_C"))
    (for _array_element _outactors
      (Utilities|Map|Add (Variables|Default|GetSpawnPoints) (Default|GetPlayerIndex _array_element) _array_element))))
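; Player controller for turn-based battles that tracks whether it is the player's turn and passes turn actions to the game mode.
; On the local controller it creates the DetermineTurn widget at BeginPlay.
; StartTurn and EndTurn set the turn flag and broadcast OnPlayerTurnChange.
; Enter during the player's turn triggers the attack action, which only calls CycleTurn on TurnBasedGM.
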(event Custom|StartTurn
  (CallFunction|SetPlayerTurn true))

(event Custom|EndTurn
  (CallFunction|SetPlayerTurn false))

(event Custom|Action%20-%20Attack
  (bind _asturn_based_gm (Utilities|Casting|CastToTurnBasedGM (Game|GetGameMode)))
  (Default|CycleTurn _asturn_based_gm))

(event EventBeginPlay
  (if (Pawn|IsLocalController)
    (bind _returnvalue (UserInterface|CreateWidget "/Game/BattleBP/Blueprints/Battle/widgets/DetermineTurn.DetermineTurn_C" self))
    (UserInterface|Viewport|AddtoViewport _returnvalue 0)))

(event EventTick
  (params (DeltaSeconds :type Float%20%28single-precision%29)))

(event Input|KeyboardEvents|SpaceBar
  (params (Key :type Key%20Structure :default "None")))

(event Input|KeyboardEvents|Enter
  (params (Key :type Key%20Structure :default "None"))
  (:Pressed
    (if (Variables|Default|GetplayerTurn)
      (CallFunction|TurnButton))))

(fn ConstructionScript)

(fn SetPlayerTurn
  (params (PlayerTurn :type Boolean))
  (bind _output_get (Variables|Default|SetplayerTurn PlayerTurn))
  (Default|CallOnPlayerTurnChange _output_get))

(fn TurnButton
  (CallFunction|Action-Attack))